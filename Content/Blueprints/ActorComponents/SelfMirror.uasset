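; SelfMirror is an actor component that shows and hides a mirror for an IK_Pawn owner.
; Show spawns a BP_3x_Mirror at the world transform of the pawn's Mirror component, unless a valid one already exists.
; Hide destroys the spawned mirror, and the EndPlay and component-deactivated events run the same cleanup.
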(event `Show`
  (bind _asik_pawn (cast `/DynamicalSystems/FullBodyIK/Blueprints/IK_Pawn` (`self.GetOwner`)))
  (`/Engine/EditorBlueprintResources/StandardMacros.IsValid` (`self.Mirror`)
    (:`Is Not Valid`
      (bind _returnvalue (`|SpawnActorFromClass` "/Game/Core/UI/3D/Mirrors/BP_3x_Mirror.BP_3x_Mirror_C" (`SceneComponent.K2_GetComponentToWorld` (`/DynamicalSystems/FullBodyIK/Blueprints/IK_Pawn.Mirror` _asik_pawn)) "AlwaysSpawn" "OverrideRootScale" null null))
      (set `self.Mirror` _returnvalue))))

(event `Hide`
  (bind _mirror (`self.Mirror`))
  (`/Engine/EditorBlueprintResources/StandardMacros.IsValid` _mirror :!label _label
    (:`Is Valid`
      (`Actor.K2_DestroyActor` _mirror))))

(event `self.ReceiveEndPlay`
  (params (EndPlayReason :type "EEndPlayReason Enum" :default "Destroyed"))
  (goto _label))

(event `OnComponentDeactivated_Event`
  (params (Component :type "ActorComponent Object Reference"))
  (goto _label))