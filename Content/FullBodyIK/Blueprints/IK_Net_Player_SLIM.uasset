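; Player-side network class for the full-body IK pawn, handling a replicated avatar pose snapshot for remote display.
; BeginPlay captures an initial snapshot from the controlled IK_Pawn_SLIM's avatar mesh.
; The Snapshot rep-notify restores bone names, mesh name, snapshot name and validity from that local copy, leaving transforms untouched.
; SetPawnPose, not called within this class, passes the snapshot to the pawn's ABP_Remote_Phase anim instance.
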(event EventBeginPlay
  (bind _asik_pawn_slim (Utilities|Casting|CastToIK_Pawn_SLIM (Pawn|GetControlledPawn)))
  (bind _skeletalmesh (Default|GetAvatarMesh _asik_pawn_slim))
  (Class|SkeletalMeshComponent|SnapshotPose _skeletalmesh (Variables|Default|GetInitialSnapshot)))

(fn ConstructionScript)

(fn GetState
  (bind _playerstate (Variables|Default|GetPlayerState))
  (bind (_asavatar_state _bsuccess) (Utilities|Casting|CastToAvatarState _playerstate))
  (return _asavatar_state _bsuccess))

(fn OnRepSnapshot
  (bind _initialsnapshot (Variables|Default|GetInitialSnapshot))
  (Utilities|Struct|SetmembersinPoseSnapshot (Variables|Default|GetSnapshot) (.bonenames _initialsnapshot) (.skeletalmeshname _initialsnapshot) (.snapshotname _initialsnapshot) (.bisvalid _initialsnapshot)))

(fn SetPawnPose
  (bind _skeletalmesh (Class|IKAvatar|GetAvatarMesh(Message) (Pawn|GetControlledPawn)))
  (bind _asabp_remote_phase (Utilities|Casting|CastToABP_Remote_Phase (Components|SkeletalMesh|GetAnimInstance _skeletalmesh)))
  (Default|SetPose _asabp_remote_phase (Variables|Default|GetSnapshot)))