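; Player controller for a full-body IK VR avatar, setting floor tracking and linking the player to their IK pawn.
; Tick retries Validation until it resolves the pawn, spawns an IK camera and caches both motion controllers.
; Input triggers HMD height calibration and writes grip values to AvatarState.
; Helpers for gravity, locomotion and copying IK transforms to AvatarState are not called here, and much older grip-climbing and floor logic is disconnected or deprecated.
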(event `self.ReceiveBeginPlay`
  (`|ExecutionSequence`
    (:`then_0`
      (`HeadMountedDisplayFunctionLibrary.SetTrackingOrigin` "Floor"))
    (:`then_1`
      (set `self.MovementAllowed` true))))

(event `Spawned`
  (params (Camera :type "/DynamicalSystems/FullBodyIK/Blueprints/IK_Camera Object Reference") (Pawn :type "/DynamicalSystems/FullBodyIK/Blueprints/IK_Pawn Object Reference"))
  (set `self.IK_Pawn` Pawn)
  (set `self.IK_Camera` Camera))

(event `self.ReceiveTick`
  (params (DeltaSeconds :type "Float (single-precision)"))
  (`|ExecutionSequence`
    (:`then_0`
      (if (not (`self.Valid`))
        (bind _isvalid (`self.Validation`))
        (set `self.Valid` _isvalid)))))

(event `InputAction|CalibrateHeight`
  (params (Key :type "Key Structure"))
  ;[0 0 0] Calibrate Height on Controller until keyboard shows up in builds correctly.
  (:`Pressed`
    (`self.CalibrateHeight`)))

(event `self.FloorNav`
  (params (DeltaTime :type "Float (single-precision)"))
  (bind _ik_camera (`self.IK_Camera`))
  (bind _ik_pawn (`self.IK_Pawn`))
  (bind _defaultsceneroot (`/DynamicalSystems/FullBodyIK/Blueprints/IK_Camera.DefaultSceneRoot` (`self.IK_Camera`)))
  (bind _returnvalue (`SceneComponent.K2_GetComponentLocation` (`/DynamicalSystems/FullBodyIK/Blueprints/IK_Pawn.DefaultSceneRoot` (`self.IK_Pawn`))))
  (bind (_returnvalue_x _returnvalue_y _returnvalue_z) (`KismetMathLibrary.BreakVector` (`SceneComponent.K2_GetComponentLocation` (`/DynamicalSystems/FullBodyIK/Blueprints/IK_Camera.DefaultSceneRoot` _ik_camera))))
  (bind (_returnvalue_x_2 _returnvalue_y_2 _returnvalue_z_2) (`KismetMathLibrary.BreakVector` (`SceneComponent.K2_GetComponentLocation` (`/DynamicalSystems/FullBodyIK/Blueprints/IK_Pawn.DefaultSceneRoot` (`self.IK_Pawn`)))))
  (bind (_returnvalue_x_3 _returnvalue_y_3) (`KismetMathLibrary.BreakVector` (`SceneComponent.K2_GetComponentLocation` _defaultsceneroot)))
  (bind _x (.x (`SceneComponent.K2_GetComponentLocation` (`/DynamicalSystems/FullBodyIK/Blueprints/IK_Pawn.DefaultSceneRoot` _ik_pawn))))
  (bind _y (.y (`SceneComponent.K2_GetComponentLocation` (`/DynamicalSystems/FullBodyIK/Blueprints/IK_Pawn.DefaultSceneRoot` _ik_pawn))))
  (bind _z (.z (`SceneComponent.K2_GetComponentLocation` (`/DynamicalSystems/FullBodyIK/Blueprints/IK_Pawn.DefaultSceneRoot` _ik_pawn))))
  (if (and (`KismetSystemLibrary.IsValid` _ik_camera) (`KismetSystemLibrary.IsValid` _ik_pawn))
    (set `self.HeadOffset_0` (- _returnvalue_z _z))
    (bind (_outhit _returnvalue_2) (`KismetSystemLibrary.LineTraceSingleForObjects` (`KismetMathLibrary.MakeVector` _x _y (+ _z 100.0)) (`KismetMathLibrary.MakeVector` _x _y (+ _z -20000.0)) (`|MakeArray` "ObjectTypeQuery1" "ObjectTypeQuery14" "ObjectTypeQuery10" :!type "EObjectTypeQuery Enum") false (`|MakeArray` (`self.IK_Pawn`) :!type "Actor Object Reference")))
    (if _returnvalue_2
      (bind (_bblockinghit _binitialoverlap _time _distance _location _impactpoint _normal) (`GameplayStatics.BreakHitResult` _outhit))
      (`SceneComponent.K2_SetWorldLocation` (`/DynamicalSystems/FullBodyIK/Blueprints/IK_Pawn.DefaultSceneRoot` (`self.IK_Pawn`)) (`KismetMathLibrary.VInterpTo` _returnvalue _location DeltaTime (`KismetMathLibrary.MapRangeClamped` (.z (- _location _returnvalue)) 50.0 -50.0 (* 1.0 20.0) (* (`self.Gravity`) 1.0))) false false)
      (bind _output_get (set `/DynamicalSystems/FullBodyIK/Blueprints/IK_Pawn.Floor` (.z _location) (`self.IK_Pawn`)))
      (`SceneComponent.K2_SetWorldLocation` _defaultsceneroot (`KismetMathLibrary.MakeVector` _returnvalue_x_3 _returnvalue_y_3 (+ (`self.HeadOffset_0`) _returnvalue_z_2)) false false))))

(event `self.Latch`
  (params (DeltaTime :type "Float (single-precision)")))

(event `self.CalibrateHeight`
  (bind _asik_pawn_slim (cast `/DynamicalSystems/FullBodyIK/Blueprints/IK_Pawn_SLIM` (`self.IK_Pawn`)))
  (`/DynamicalSystems/FullBodyIK/Blueprints/IK_Pawn_SLIM.SetHeightFromHMD` _asik_pawn_slim))

(event `InputAction|AvatarHeight` :consume false
  (params (Key :type "Key Structure"))
  (:`Pressed`
    (`self.CalibrateHeight`)))

(event `UpdateFromState`
  (params (delta :type "Float (double-precision)")))

(event `InputAxisKey|MotionController_Left_TriggerAxis` :consume false
  (params (AxisValue :type "Float (single-precision)"))
  ;[1 1 1] Dont hard code.
)

(event `InputAxis|GripLeft`
  (params (AxisValue :type "Float (single-precision)"))
  (bind (_asavatar_state _success) (`self.GetState`))
  (if _success
    (set `/DynamicalSystems/State/AvatarState.LeftHandGripping` AxisValue _asavatar_state)))

(event `InputAxis|GripRight`
  (params (AxisValue :type "Float (single-precision)"))
  (bind (_asavatar_state _success) (`self.GetState`))
  (if _success
    (set `/DynamicalSystems/State/AvatarState.RightHandGripping` AxisValue _asavatar_state)))

(event `InputAxisKey|MotionController_Right_TriggerAxis` :consume false
  (params (AxisValue :type "Float (single-precision)"))
  ;[1 1 1] Dont hard code.
)

(fn `ApplyGravity`
  (params (Distance :type "Float (double-precision)") (DeltaTime :type "Float (double-precision)"))
  (bind _asik_pawn_slim (cast `/DynamicalSystems/FullBodyIK/Blueprints/IK_Pawn_SLIM` (`self.IK_Pawn`)))
  (bind (_distance _returnvalue _trans _outhit) (`self.TraceForFloor`))
  (if _returnvalue
    (set `/DynamicalSystems/State/AvatarState.Floor` _trans (`self.GetState`))
    (bind _origin (`/DynamicalSystems/FullBodyIK/Blueprints/IK_Pawn_SLIM.Origin` _asik_pawn_slim))
    (bind _returnvalue_2 (`SceneComponent.K2_GetComponentLocation` _origin))
    (`SceneComponent.K2_SetWorldLocation` _origin (`KismetMathLibrary.VInterpTo` _returnvalue_2 (`.Location` (`GameplayStatics.BreakHitResult` _outhit)) DeltaTime) false false)
    (else
      (`SceneComponent.K2_SetWorldLocation` _origin (+ _returnvalue_2 (* (0.0 0.0 -1.0) (* DeltaTime (`self.Gravity`)))) false false))))

(fn `GetState`
  (returns (`AsAvatar State` :type "/DynamicalSystems/State/AvatarState Object Reference") (Success :type Boolean))
  (bind _asavatar_state (cast `/DynamicalSystems/State/AvatarState` (`self.PlayerState`))
    (:`then`
      _)
    (:`CastFailed`
      _))
  (return _asavatar_state (`KismetSystemLibrary.IsValid` _asavatar_state)))

(fn `TraceForFloor`
  (returns (Distance :type "Float (double-precision)") (ReturnValue :type Boolean) (Trans :type "Transform Structure") (OutHit :type "HitResult Structure"))
  (bind _asik_pawn_slim (cast `/DynamicalSystems/FullBodyIK/Blueprints/IK_Pawn_SLIM` (`self.IK_Pawn`)))
  (if (`.Success` (`self.GetState`))
    (bind _location (.location (`SceneComponent.K2_GetComponentToWorld` (`/DynamicalSystems/FullBodyIK/Blueprints/IK_Pawn_SLIM.HMDCamera` _asik_pawn_slim))))
    (bind (_outhit _returnvalue) (`KismetSystemLibrary.LineTraceSingle` :`Start` _location :`End` (- _location (0.0 0.0 25.0)) :`TraceChannel` "TraceTypeQuery3" :`DrawDebugType` "ForOneFrame" :`TraceColor` (struct :`G` 0.998362 :`B` 1.0 :`A` 1.0) :`TraceHitColor` (struct :`G` 0.261996 :`B` 1.0 :`A` 1.0)))
    (bind (_bblockinghit _binitialoverlap _time _distance _location_2) (`GameplayStatics.BreakHitResult` _outhit))
    (return _distance _returnvalue (`KismetMathLibrary.MakeTransform` _location_2 (`KismetMathLibrary.FindLookAtRotation` (* (+ _location (* (`KismetMathLibrary.GetForwardVector` (.rotation (`SceneComponent.K2_GetComponentToWorld` (`/DynamicalSystems/FullBodyIK/Blueprints/IK_Pawn_SLIM.HMDCamera` _asik_pawn_slim)))) 500.0)) (1.0 1.0 0.0)) (`self.K2_GetActorLocation` _asik_pawn_slim)) (.scale (`SceneComponent.K2_GetComponentToWorld` (`/DynamicalSystems/FullBodyIK/Blueprints/IK_Pawn_SLIM.HMDCamera` _asik_pawn_slim)))) _outhit)))

(fn `TraceForGround`)

(fn `UserConstructionScript`
  (`parent.UserConstructionScript`)
  (`ActorComponent.K2_DestroyComponent` (`self.LeapOverride`)))

(fn `Validation`
  (returns (IsValid :type Boolean))
  (bind _ik_pawn (`self.IK_Pawn`))
  (bind _ik_pawn_2 (`self.IK_Pawn`))
  (`|ExecutionSequence`
    (:`then_0`
      (`/Engine/EditorBlueprintResources/StandardMacros.IsValid` (`self.IK_Pawn`)
        (:`Is Not Valid`
          (bind _asik_pawn (cast `/DynamicalSystems/FullBodyIK/Blueprints/IK_Pawn` (`self.K2_GetPawn`))
            (:`then`
              (bind _output_get (set `self.IK_Pawn` _asik_pawn))
              (`self.SetOwner` _output_get self))
            (:`CastFailed`
              (return false))))))
    (:`then_1`
      (`/Engine/EditorBlueprintResources/StandardMacros.IsValid` (`self.IK_Camera`)
        (:`Is Not Valid`
          (`/Engine/EditorBlueprintResources/StandardMacros.IsValid` _ik_pawn
            (:`Is Valid`
              (bind _returnvalue (`|SpawnActorFromClass` "/DynamicalSystems/FullBodyIK/Blueprints/IK_Camera.IK_Camera_C" (`SceneComponent.K2_GetComponentToWorld` (`/DynamicalSystems/FullBodyIK/Blueprints/IK_Pawn.DefaultSceneRoot` _ik_pawn)) "AlwaysSpawn" "OverrideRootScale" _ik_pawn null))
              (bind _output_get_2 (set `self.IK_Camera` _returnvalue))
              (`self.SetViewTargetWithBlend` self (`self.IK_Pawn`) 0.0 "VTBlend_Linear" 0.0 false)
              (`|ExecutionSequence`
                (:`then_0`
                  (bind _asik_motion_controller (cast `/DynamicalSystems/FullBodyIK/Blueprints/IK_MotionController` (`ChildActorComponent.ChildActor` (`/DynamicalSystems/FullBodyIK/Blueprints/IK_Pawn.ChildMotionControllerL` _ik_pawn_2)))
                    (:`then`
                      (set `self.IK_MotionControllerL` _asik_motion_controller))
                    (:`CastFailed`
                      (return false))))
                (:`then_1`
                  (bind _asik_motion_controller_2 (cast `/DynamicalSystems/FullBodyIK/Blueprints/IK_MotionController` (`ChildActorComponent.ChildActor` (`/DynamicalSystems/FullBodyIK/Blueprints/IK_Pawn.ChildMotionControllerR` _ik_pawn_2)))
                    (:`then`
                      (set `self.IK_MotionControllerR` _asik_motion_controller_2))
                    (:`CastFailed`
                      (return false))))))
            (:`Is Not Valid`
              (return false))))))
    (:`then_3`
      (return true))))