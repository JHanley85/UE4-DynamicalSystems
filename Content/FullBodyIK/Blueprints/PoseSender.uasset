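; PoseSender is an experimental actor for sharing a skeletal mesh pose over the network with PlaybackBot actors.
; SendPose snapshots the mesh and copies bone names and other metadata, without transforms, into InitialSnapshot.
; A rep-notify function restores that metadata onto Snapshot and passes it to every PlaybackBot found at construction.
; The custom NetClient send paths are disconnected, leaving only RPC ID debug prints and empty test events.
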(event `self.ReceiveBeginPlay`
  (`OSSFunctionLibrary.PrintRPCID` (`|CreateDelegate` :!event `TestRPCId`)))

(event `self.ReceiveTick`
  (params (DeltaSeconds :type "Float (single-precision)")))

(event `Send Pose`
  (bind (_localtransforms _bonenames _skeletalmeshname _snapshotname _bisvalid) (break `PoseSnapshot` (`self.snapshot`)))
  (`SkeletalMeshComponent.SnapshotPose` (`self.Mesh`) (`self.snapshot`))
  (setmembers `PoseSnapshot` :`StructRef` (`self.InitialSnapshot`) :`BoneNames` _bonenames :`SkeletalMeshName` _skeletalmeshname :`SnapshotName` _snapshotname :`bIsValid` _bisvalid))

(event `OnEndPlay_Event_0`
  (params (Actor :type "Actor Object Reference") (EndPlayReason :type "EEndPlayReason Enum" :default "Destroyed")))

(event `OnRep_Snapshit`
  (params (InBytes :type "Array of Byte")))

(event `TestRPCId`
  (params (NewParam :type "PoseSnapshot Structure")))

(event `TEst2`
  (params (NewParam :type "PoseSnapshot Structure")))

(fn `OnRep_NewVar_0`
  (bind (_localtransforms _bonenames _skeletalmeshname _snapshotname _bisvalid) (break `PoseSnapshot` (`self.InitialSnapshot`)))
  (bind _structout (setmembers `PoseSnapshot` :`StructRef` (`self.snapshot`) :`BoneNames` _bonenames :`SkeletalMeshName` _skeletalmeshname :`SnapshotName` _snapshotname :`bIsValid` _bisvalid))
  (`self.OnSnapshot` _structout))

(fn `OnSnapshot`
  (params (Shnappshot :type "PoseSnapshot Structure"))
  (for _array_element (`self.Playback bots`)
    (`/Game/Dancers/Bots/PlaybackBot.OnPoseUpdate` _array_element Shnappshot))
  (return))

(fn `UserConstructionScript`
  (`|ExecutionSequence`
    (:`then_0`
      (bind _outactors (`GameplayStatics.GetAllActorsOfClass` "/Script/DynamicalSystems.NetClient"))
      (set `self.Client` (`/MidiManagerPlugin/NewMacroLibrary.GetLast` _outactors))
      (bind _outactors_2 (`GameplayStatics.GetAllActorsOfClass` "/Game/Dancers/Bots/PlaybackBot.PlaybackBot_C"))
      (set `self.Playback bots` _outactors_2))
    (:`then_1`
      (`OSSFunctionLibrary.PrintRPCID` (`|CreateDelegate` :!event `TEst2`))
      (`OSSFunctionLibrary.PrintRPCID` (`|CreateDelegate` :!event `TestRPCId`)))))