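; Blueprint utility library for full-body IK avatars driven by an HMD and motion controllers.
; Avatar functions look up data table rows by index or name, then apply the loaded mesh, anim class and materials to a skeletal mesh component.
; MeasureAvatar derives height and headset and controller offsets from mesh sockets.
; Helpers trace vertically at foot sockets for ground offset, rotate points around pivots, and debug-draw cubic Bezier curves.
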(fn `DebugDrawCubicBezier`
  (params (Time :type "Float (double-precision)") (P0 :type "Vector Structure") (P1 :type "Vector Structure") (P2 :type "Vector Structure") (P3 :type "Vector Structure"))
  (bind _returnvalue (`KismetMathLibrary.Conv_IntToDouble` 30))
  (for _index (range 30)
    (`KismetSystemLibrary.DrawDebugLine` null (`DynamicalUtil.CubicBezier` (/ (`KismetMathLibrary.Conv_IntToDouble` _index) _returnvalue) P0 P1 P2 P3) (`DynamicalUtil.CubicBezier` (/ (`KismetMathLibrary.Conv_IntToDouble` (+ _index 1)) _returnvalue) P0 P1 P2 P3) (struct :`R` 1.0 :`G` 0.887345 :`A` 1.0) 0.0 1.0))
  (`|ExecutionSequence`
    (:`then_0`
      (`KismetSystemLibrary.DrawDebugArrow` null P0 P1 2.0 (struct :`R` 1.0 :`B` 0.654823 :`A` 1.0) 0.0 1.0))
    (:`then_1`
      (`KismetSystemLibrary.DrawDebugArrow` null P3 P2 2.0 (struct :`G` 0.573642 :`B` 1.0 :`A` 1.0) 0.0 1.0))))

(fn `GetAvatarFromTable`
  (params (Id :type Integer))
  (returns (Data :type "/DynamicalSystems/FullBodyIK/Characters/Mannequin/AvatarData Structure") (Success :type Boolean) (tableref :type "DataTable Object Reference"))
  (bind _returnvalue (`DynamicalSystemsSettings.GetAvatarTable`))
  (`/Engine/EditorBlueprintResources/StandardMacros.IsValid` _returnvalue
    (:`Is Valid`
      (bind _outrownames (`DataTableFunctionLibrary.GetDataTableRowNames` _returnvalue))
      (bind _returnvalue_2 (`KismetArrayLibrary.Array_Length` _outrownames))
      (bind _returnvalue_3 (`KismetMathLibrary.Min` _returnvalue_2 Id))
      (if (> _returnvalue_2 _returnvalue_3)
        (bind _returnvalue_4 (`|GetDataTableRow` _returnvalue (`|GetArrayItem` _outrownames _returnvalue_3))
          (:`then`
            (`KismetSystemLibrary.PrintText` null (`|FormatText` "Found Avatar ID {i} [{x}]" _returnvalue_3 (`KismetTextLibrary.Conv_StringToText` (`KismetSystemLibrary.Conv_SoftObjectReferenceToString` (`.Mesh_26_D2A02CD1466D9A701F59CA99BC45CE35` (break `/DynamicalSystems/FullBodyIK/Characters/Mannequin/AvatarData` _returnvalue_4))))) false false)
            (return _returnvalue_4 true _returnvalue))
          (:`RowNotFound`
            (`KismetSystemLibrary.PrintString` (`local.__WorldContext`) "row not found" false)
            (return (struct) false _returnvalue)))
        (else
          (`KismetSystemLibrary.PrintString` (`local.__WorldContext`) "No such index in table" false)
          (return (struct) false _returnvalue))))
    (:`Is Not Valid`
      (`KismetSystemLibrary.PrintString` (`local.__WorldContext`) "Not a table.")
      (return (struct) false null))))

(fn `GetOrbitPositionAroundLocation`
  (params (BaseLocation :type "Vector Structure") (RelativePivot :type "Vector Structure") (Rotation :type "Rotator Structure"))
  (returns (TargetLocation :type "Vector Structure") (TargetRotation :type "Rotator Structure"))
  (return (+ RelativePivot (`KismetMathLibrary.GreaterGreater_VectorRotator` (- BaseLocation RelativePivot) Rotation)) Rotation))

(fn `IK_FootTrace`
  (params (SKMesh :type "SceneComponent Object Reference") (InSocketName :type Name) (Scale :type "Float (double-precision)") (TraceDistance :type "Float (double-precision)"))
  (returns (Offset :type "Float (double-precision)") (ReturnValue :type Boolean) (Location :type "Vector Structure"))
  (bind _returnvalue (`SceneComponent.GetSocketLocation` SKMesh InSocketName))
  (bind (_outhit _returnvalue_2) (`KismetSystemLibrary.LineTraceSingle` SKMesh (+ _returnvalue (`KismetMathLibrary.MakeVector` 0.0 0.0 TraceDistance)) (- _returnvalue (`KismetMathLibrary.MakeVector` 0.0 0.0 TraceDistance)) "TraceTypeQuery3" true (`|MakeArray` (`ActorComponent.GetOwner` SKMesh)) "None" true (struct :`G` 1.0 :`B` 0.207271 :`A` 1.0) (struct :`R` 1.0 :`G` 0.066323 :`A` 1.0)))
  (bind (_bblockinghit _binitialoverlap _time _distance _location) (`GameplayStatics.BreakHitResult` _outhit))
  (return (`KismetMathLibrary.SelectFloat` (.z (- _returnvalue _location)) 0.0 _bblockinghit) _returnvalue_2 (`KismetMathLibrary.SelectVector` _location _returnvalue _bblockinghit)))

(fn `MeasureAvatar`
  (params (Mesh :type "SkeletalMeshComponent Object Reference (by ref)") (height :type "Float (double-precision) (by ref)") (HMDOffset :type "Transform Structure (by ref)") (LeftMotionControllerOffset :type "Transform Structure (by ref)") (RightMotionControllerOffset :type "Transform Structure (by ref)") (AvatarData :type "/DynamicalSystems/FullBodyIK/Characters/Mannequin/AvatarData Structure"))
  (returns (outheight :type "Float (double-precision)"))
  (bind (_mesh _animinstance _headsocket _lmotioncontrollersocket _rmotioncontrollersocket _lfootsocket _rfootsocket _floorsocket) (break `/DynamicalSystems/FullBodyIK/Characters/Mannequin/AvatarData` AvatarData))
  (bind _returnvalue (`KismetMathLibrary.VSize` (- (* (`SceneComponent.GetSocketLocation` Mesh _headsocket) (0.0 0.0 1.0)) (* (`SceneComponent.GetSocketLocation` Mesh _floorsocket) (0.0 0.0 1.0)))))
  (`|ExecutionSequence`
    (:`then_0`
      (`|VariableSetRef` height _returnvalue)
      (`KismetSystemLibrary.PrintString` null (`KismetStringLibrary.Concat_StrStr` "height " (`KismetStringLibrary.Conv_DoubleToString` _returnvalue)) false false))
    (:`then_1`
      (`|VariableSetRef` HMDOffset (`SceneComponent.GetSocketTransform` Mesh _headsocket "RTS_ParentBoneSpace")))
    (:`then_2`
      (`|VariableSetRef` LeftMotionControllerOffset (`SceneComponent.GetSocketTransform` Mesh _lmotioncontrollersocket "RTS_ParentBoneSpace")))
    (:`then_3`
      (`|VariableSetRef` RightMotionControllerOffset (`SceneComponent.GetSocketTransform` Mesh _rmotioncontrollersocket "RTS_ParentBoneSpace")))
    (:`then_4`
      (return _returnvalue))))

(fn `SetAvatar`
  (params (AvatarData :type "/DynamicalSystems/FullBodyIK/Characters/Mannequin/AvatarData Structure") (Target :type "SkeletalMeshComponent Object Reference (by ref)"))
  (bind (_mesh _animinstance) (break `/DynamicalSystems/FullBodyIK/Characters/Mannequin/AvatarData` AvatarData))
  (`/Engine/EditorBlueprintResources/StandardMacros.IsValid` Target
    (:`Is Valid`
      (bind _returnvalue (`DynamicalSystemsSettings.LoadMesh` (`KismetSystemLibrary.MakeSoftObjectPath` (`KismetSystemLibrary.Conv_SoftObjectReferenceToString` _mesh))))
      (`KismetSystemLibrary.PrintString` null (`KismetStringLibrary.Conv_ObjectToString` _returnvalue))
      (`SkinnedMeshComponent.SetSkinnedAssetAndUpdate` Target _returnvalue true)
      (`SkeletalMeshComponent.SetAnimInstanceClass` Target _animinstance)
      (for (_array_element _array_index) (`SkeletalMesh.Materials` _returnvalue)
        (`PrimitiveComponent.SetMaterial` Target _array_index (`.MaterialInterface` (break `SkeletalMaterial` _array_element)))
        (`KismetSystemLibrary.PrintText` (`local.__WorldContext`) (`|FormatText` "Avatar {name} w/ anim {anim}" (`KismetTextLibrary.Conv_StringToText` (`KismetSystemLibrary.GetObjectName` _returnvalue)) (`KismetTextLibrary.Conv_StringToText` (`KismetSystemLibrary.GetClassDisplayName` _animinstance))) false))
      (return))))

(fn `SetAvatarByName`
  (params (ItemToFind :type "Name (by ref)") (Pawn :type "Pawn Object Reference"))
  (bind ___worldcontext (`local.__WorldContext`))
  (bind _returnvalue (`DynamicalSystemsSettings.GetAvatarTable`))
  (bind _outrownames (`DataTableFunctionLibrary.GetDataTableRowNames` _returnvalue))
  (bind _returnvalue_2 (`KismetArrayLibrary.Array_Find` _outrownames ItemToFind))
  (if (> _returnvalue_2 -1)
    (bind _data (`self.GetAvatarFromTable` _returnvalue_2 ___worldcontext))
    (bind _skeletalmesh (message `/DynamicalSystems/Blueprints/Interfaces/IKAvatar.GetAvatarMesh` Pawn))
    (`self.SetAvatar` _data _skeletalmesh ___worldcontext)))